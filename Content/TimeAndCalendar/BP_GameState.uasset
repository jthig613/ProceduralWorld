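; Game state Blueprint that runs the in-game clock and calendar.
; On BeginPlay it seeds GameTime in hours; each Tick while GameSpeed is non-zero, a CalculateGameTime library call advances it and yields a day counter.
; UpdateClockCalendar derives hours, minutes and seconds through chained remainder divisions and rolls day, month and year over by month length.
; The result fills a DateTime struct, which is printed on screen for debugging.
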(event Custom|CalculateTime
  (params (DeltaTime :type Float%20%28double-precision%29))
  (Variables|GameSpeedSettings|SetGameTime (.OutGameTime (CallFunction|CalculateGameTime DeltaTime (Variables|GameSpeedSettings|GetGameSpeed) (Variables|GameSpeedSettings|GetGameTime))))
  (Variables|Calendar|SetDayCounter (.DayCounter (CallFunction|CalculateGameTime DeltaTime (Variables|GameSpeedSettings|GetGameSpeed) (Variables|GameSpeedSettings|GetGameTime)))))

(event Custom|SetClockCalendar
  (bind _datetimestruct (Variables|GameSpeedSettings|GetDateTimeStruct))
  (bind (_year _month _day _hour _minute _second) (Math|DateTime|BreakDateTime _datetimestruct))
  (bind (_year_2 _month_2 _day_2 _hours _minutes _seconds) (GameTime|UpdateClockCalendar))
  (CallFunction|SetDateTimeStruct _year_2 _month_2 _day_2 _hours _minutes _seconds)
  (CallFunction|DebugTime _hour _minute _second _month _day _year))

(event EventBeginPlay
  (GameSpeedSettings|SetInitialGameTime))

(event EventTick
  (params (DeltaSeconds :type Float%20%28single-precision%29))
  (if (!= (Variables|GameSpeedSettings|GetGameSpeed) 0.0)
    (CallFunction|CalculateTime DeltaSeconds)
    (CallFunction|SetClockCalendar)))

(fn ConstructionScript)

(fn SetInitialGameTime
  (Variables|GameSpeedSettings|SetGameTime (+ (Variables|Clock|GetHours) (/ (Variables|Clock|GetMinutes) 6e+01) (/ (Variables|Clock|GetSeconds) 3.6e+03))))

(fn UpdateClockCalendar
  (bind _gametime (Variables|GameSpeedSettings|GetGameTime))
  (bind _returnvalue (* _gametime 3.6e+03))
  (bind (_remainder _returnvalue_2) (Math|Float|Division(WholeandRemainder) _returnvalue 6e+01))
  (bind _returnvalue_3 (Math|Conversions|ToFloat(Integer) _returnvalue_2))
  (bind (_remainder_2 _returnvalue_4) (Math|Float|Division(WholeandRemainder) _returnvalue_3 6e+01))
  ;[1 1 1] Set Seconds
  (Variables|Clock|SetSeconds (Math|Float|Floor _remainder))
  ;[1 1 1] Set Minutes
  (Variables|Clock|SetMinutes (Math|Float|Floor _remainder_2))
  ;[1 1 1] Set Hours
  (Variables|Clock|SetHours (Math|Float|Floor (.Remainder (Math|Float|Division(WholeandRemainder) (Math|Conversions|ToFloat(Integer) _returnvalue_4) 24.0))))
  ;[1 1 1] Calendar
  (bind _output_get (Variables|Calendar|SetDay (+ (Variables|Calendar|GetDay) (Variables|Calendar|GetDayCounter))))
  (if (> _output_get (Class|KismetMathLibrary|DaysinMonth (Variables|Calendar|GetYear) (Variables|Calendar|GetMonth)))
    (Variables|Calendar|SetDay 1)
    (Variables|Calendar|SetMonth (+ (Variables|Calendar|GetMonth) 1)))
  (if (> (Variables|Calendar|GetMonth) 12)
    (Variables|Calendar|SetMonth 1)
    (Variables|Calendar|SetYear (+ (Variables|Calendar|GetYear) 1)))
  (return (Variables|Calendar|GetYear) (Variables|Calendar|GetMonth) (Variables|Calendar|GetDay) (Variables|Clock|GetHours) (Variables|Clock|GetMinutes) (Variables|Clock|GetSeconds)))

(fn SetDateTimeStruct
  (params (Year :type Integer%20%28by%20ref%29) (Month :type Integer%20%28by%20ref%29) (Day :type Integer%20%28by%20ref%29) (Hour :type Integer%20%28by%20ref%29) (Minute :type Integer%20%28by%20ref%29) (Second :type Integer%20%28by%20ref%29))
  (Variables|GameSpeedSettings|SetDateTimeStruct (Math|DateTime|MakeDateTime Year Month Day Hour Minute Second)))

(fn DebugTime
  (params (Hour :type Integer%20%28by%20ref%29) (Minute :type Integer%20%28by%20ref%29) (Second :type Integer%20%28by%20ref%29) (Month :type Integer%20%28by%20ref%29) (Day :type Integer%20%28by%20ref%29) (Year :type Integer%20%28by%20ref%29))
  (Development|PrintString (Utilities|String|Append (Utilities|String|ToString(Integer) Hour) ":" (Utilities|String|ToString(Integer) Minute) ":" (Utilities|String|ToString(Integer) Second) "      " (Utilities|String|ToString(Integer) Month) "/" (Utilities|String|ToString(Integer) Day) "/" (Utilities|String|ToString(Integer) Year)) true true "(R=0.000000,G=0.660000,B=1.000000,A=1.000000)" 2.0 "1"))